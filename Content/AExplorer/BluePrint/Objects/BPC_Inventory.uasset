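; BPC_Inventory is an inventory component that holds items in a slot array.
; SetSizeInventory stores the new size, clears any existing slots, discarding their contents, and refills the array with a loop over that size.
; MoveItem swaps the contents of two slot indices through a temporary item.
; It has no active BeginPlay or Tick logic.
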(fn `MoveItem`
  (params (InvIndexToMove :type Byte) (InvIndexItem :type Byte))
  (locals (TempItem :type "/Game/AExplorer/BluePrint/Objects/BP_Item Object Reference"))
  (bind _returnvalue (`KismetMathLibrary.Conv_ByteToInt` InvIndexItem))
  (bind _returnvalue_2 (`KismetMathLibrary.Conv_ByteToInt` InvIndexToMove))
  (bind _slots (`self.Slots`))
  (bind _output_get (set `local.TempItem` (`|GetArrayItem` _slots _returnvalue_2)))
  (`KismetArrayLibrary.Array_Set` _slots _returnvalue_2 (`|GetArrayItem` _slots _returnvalue))
  (`KismetArrayLibrary.Array_Set` _slots _returnvalue _output_get))

(fn `SetSizeInventory`
  (params (newSize :type Integer))
  (bind _slots (`self.Slots`))
  (set `self.sizeInventory` newSize)
  (if (`KismetArrayLibrary.Array_IsNotEmpty` (`self.Slots`))
    (`KismetArrayLibrary.Array_Clear` _slots))
  (for _ (range (+ (`self.sizeInventory`) 1))
    (`KismetArrayLibrary.Array_Add` _slots)))