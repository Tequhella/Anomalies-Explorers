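; Interactive door that shows a tutorial prompt and takes key input while the top-down character stands near it.
; Sphere overlap with the character toggles the DidacticielDoor prompt and input for player 0, printing debug strings on enter and exit.
; Pressing F fires the OpenWrap and OpenDoorGreen calls; no door movement or open-state logic lives in this graph.
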(event `self.Sphere.OnComponentBeginOverlap`
  (params (OverlappedComponent :type "PrimitiveComponent Object Reference") (OtherActor :type "Actor Object Reference") (OtherComp :type "PrimitiveComponent Object Reference") (OtherBodyIndex :type Integer) (bFromSweep :type Boolean) (SweepResult :type "HitResult Structure (by ref)"))
  ;[1 1 1] Permet d'afficher le text au dessus de la Porte
  (cast `/Game/TopDown/Blueprints/BP_TopDownCharacter` OtherActor)
  (`SceneComponent.SetVisibility` (`self.DidacticielDoor`) true false)
  (`self.EnableInput` (`GameplayStatics.GetPlayerController` 0))
  (`KismetSystemLibrary.PrintString` "Hello"))

(event `self.Sphere.OnComponentEndOverlap`
  (params (OverlappedComponent :type "PrimitiveComponent Object Reference") (OtherActor :type "Actor Object Reference") (OtherComp :type "PrimitiveComponent Object Reference") (OtherBodyIndex :type Integer))
  ;[1 1 1] Permet d'afficher le text au dessus de la Porte
  (cast `/Game/TopDown/Blueprints/BP_TopDownCharacter` OtherActor)
  (`SceneComponent.SetVisibility` (`self.DidacticielDoor`) false false)
  (`self.DisableInput` (`GameplayStatics.GetPlayerController` 0))
  (`KismetSystemLibrary.PrintString` "je quitte"))

(event `Key|F`
  (params (Key :type "Key Structure"))
  (:`Pressed`
    (`self.OpenWrap`)
    (`self.OpenDoorGreen`)))

(fn `UserConstructionScript`)