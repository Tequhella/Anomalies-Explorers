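; Small room canvas for the dungeon generator, with twelve child-actor connection points, three each on north, south, east and west.
; Construction script and BeginPlay run identical logic, applying each point's configured state and passing it the room size derived from scaled connection-point offsets.
; Getters expose all connection points or those matching a given state.
; An overlap check on the child room collider reports collisions with other BP_RoomCollider actors.
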(event `self.ReceiveBeginPlay`
  (bind _returnvalue (`self.GetTransform` self))
  (set `self.SizeX` (* (.x (.location (`SceneComponent.GetRelativeTransform` (`self.BP_ConnectionPointNorth00`)))) (.x (.scale _returnvalue))))
  (set `self.SizeY` (* (.y (.location (`SceneComponent.GetRelativeTransform` (`self.BP_ConnectionPointEst00`)))) (.y (.scale _returnvalue))))
  (`|ExecutionSequence`
    (:`then_0`
      (`/Game/DungeonGenerator/SubLevels/Blueprint/BP_ConnectionPoint.ChangeState` (cast `/Game/DungeonGenerator/SubLevels/Blueprint/BP_ConnectionPoint` (`ChildActorComponent.ChildActor` (`self.BP_ConnectionPointNorth00`)) :!pure true) (`self.CP_N_00`))
      (`/Game/DungeonGenerator/SubLevels/Blueprint/BP_ConnectionPoint.ChangeState` (cast `/Game/DungeonGenerator/SubLevels/Blueprint/BP_ConnectionPoint` (`ChildActorComponent.ChildActor` (`self.BP_ConnectionPointSouth00`)) :!pure true) (`self.CP_S_00`))
      (`/Game/DungeonGenerator/SubLevels/Blueprint/BP_ConnectionPoint.ChangeState` (cast `/Game/DungeonGenerator/SubLevels/Blueprint/BP_ConnectionPoint` (`ChildActorComponent.ChildActor` (`self.BP_ConnectionPointEst00`)) :!pure true) (`self.CP_E_00`))
      (`/Game/DungeonGenerator/SubLevels/Blueprint/BP_ConnectionPoint.ChangeState` (cast `/Game/DungeonGenerator/SubLevels/Blueprint/BP_ConnectionPoint` (`ChildActorComponent.ChildActor` (`self.BP_ConnectionPointWest00`)) :!pure true) (`self.CP_W_00`)))
    (:`then_1`
      (`/Game/DungeonGenerator/SubLevels/Blueprint/BP_ConnectionPoint.ChangeState` (cast `/Game/DungeonGenerator/SubLevels/Blueprint/BP_ConnectionPoint` (`ChildActorComponent.ChildActor` (`self.BP_ConnectionPointNorth01`)) :!pure true) (`self.CP_N_01`))
      (`/Game/DungeonGenerator/SubLevels/Blueprint/BP_ConnectionPoint.ChangeState` (cast `/Game/DungeonGenerator/SubLevels/Blueprint/BP_ConnectionPoint` (`ChildActorComponent.ChildActor` (`self.BP_ConnectionPointSouth01`)) :!pure true) (`self.CP_S_01`))
      (`/Game/DungeonGenerator/SubLevels/Blueprint/BP_ConnectionPoint.ChangeState` (cast `/Game/DungeonGenerator/SubLevels/Blueprint/BP_ConnectionPoint` (`ChildActorComponent.ChildActor` (`self.BP_ConnectionPointEst01`)) :!pure true) (`self.CP_E_01`))
      (`/Game/DungeonGenerator/SubLevels/Blueprint/BP_ConnectionPoint.ChangeState` (cast `/Game/DungeonGenerator/SubLevels/Blueprint/BP_ConnectionPoint` (`ChildActorComponent.ChildActor` (`self.BP_ConnectionPointWest01`)) :!pure true) (`self.CP_W_01`)))
    (:`then_2`
      (`/Game/DungeonGenerator/SubLevels/Blueprint/BP_ConnectionPoint.ChangeState` (cast `/Game/DungeonGenerator/SubLevels/Blueprint/BP_ConnectionPoint` (`ChildActorComponent.ChildActor` (`self.BP_ConnectionPointNorth02`)) :!pure true) (`self.CP_N_02`))
      (`/Game/DungeonGenerator/SubLevels/Blueprint/BP_ConnectionPoint.ChangeState` (cast `/Game/DungeonGenerator/SubLevels/Blueprint/BP_ConnectionPoint` (`ChildActorComponent.ChildActor` (`self.BP_ConnectionPointSouth02`)) :!pure true) (`self.CP_S_02`))
      (`/Game/DungeonGenerator/SubLevels/Blueprint/BP_ConnectionPoint.ChangeState` (cast `/Game/DungeonGenerator/SubLevels/Blueprint/BP_ConnectionPoint` (`ChildActorComponent.ChildActor` (`self.BP_ConnectionPointEst02`)) :!pure true) (`self.CP_E_02`))
      (`/Game/DungeonGenerator/SubLevels/Blueprint/BP_ConnectionPoint.ChangeState` (cast `/Game/DungeonGenerator/SubLevels/Blueprint/BP_ConnectionPoint` (`ChildActorComponent.ChildActor` (`self.BP_ConnectionPointWest02`)) :!pure true) (`self.CP_W_02`)))
    (:`then_3`
      (bind _output_get (set `self.AllConnectionPoints` (`|MakeArray` (cast `/Game/DungeonGenerator/SubLevels/Blueprint/BP_ConnectionPoint` (`ChildActorComponent.ChildActor` (`self.BP_ConnectionPointNorth00`)) :!pure true) (cast `/Game/DungeonGenerator/SubLevels/Blueprint/BP_ConnectionPoint` (`ChildActorComponent.ChildActor` (`self.BP_ConnectionPointSouth00`)) :!pure true) (cast `/Game/DungeonGenerator/SubLevels/Blueprint/BP_ConnectionPoint` (`ChildActorComponent.ChildActor` (`self.BP_ConnectionPointEst00`)) :!pure true) (cast `/Game/DungeonGenerator/SubLevels/Blueprint/BP_ConnectionPoint` (`ChildActorComponent.ChildActor` (`self.BP_ConnectionPointWest00`)) :!pure true) (cast `/Game/DungeonGenerator/SubLevels/Blueprint/BP_ConnectionPoint` (`ChildActorComponent.ChildActor` (`self.BP_ConnectionPointNorth01`)) :!pure true) (cast `/Game/DungeonGenerator/SubLevels/Blueprint/BP_ConnectionPoint` (`ChildActorComponent.ChildActor` (`self.BP_ConnectionPointSouth01`)) :!pure true) (cast `/Game/DungeonGenerator/SubLevels/Blueprint/BP_ConnectionPoint` (`ChildActorComponent.ChildActor` (`self.BP_ConnectionPointEst01`)) :!pure true) (cast `/Game/DungeonGenerator/SubLevels/Blueprint/BP_ConnectionPoint` (`ChildActorComponent.ChildActor` (`self.BP_ConnectionPointWest01`)) :!pure true) (cast `/Game/DungeonGenerator/SubLevels/Blueprint/BP_ConnectionPoint` (`ChildActorComponent.ChildActor` (`self.BP_ConnectionPointNorth02`)) :!pure true) (cast `/Game/DungeonGenerator/SubLevels/Blueprint/BP_ConnectionPoint` (`ChildActorComponent.ChildActor` (`self.BP_ConnectionPointSouth02`)) :!pure true) (cast `/Game/DungeonGenerator/SubLevels/Blueprint/BP_ConnectionPoint` (`ChildActorComponent.ChildActor` (`self.BP_ConnectionPointEst02`)) :!pure true) (cast `/Game/DungeonGenerator/SubLevels/Blueprint/BP_ConnectionPoint` (`ChildActorComponent.ChildActor` (`self.BP_ConnectionPointWest02`)) :!pure true))))
      (for _array_element _output_get
        (set `/Game/DungeonGenerator/SubLevels/Blueprint/BP_ConnectionPoint.SizeX` (`self.SizeX`) _array_element)
        (set `/Game/DungeonGenerator/SubLevels/Blueprint/BP_ConnectionPoint.SizeY` (`self.SizeY`) _array_element)))))

(fn `GetAllConnectionPoints`
  (returns (ConnectionPoints :type "Array of /Game/DungeonGenerator/SubLevels/Blueprint/BP_ConnectionPoint Object Reference"))
  (return (`self.AllConnectionPoints`)))

(fn `GetCollisionResult`
  (returns (Overlap :type Boolean))
  (return (`KismetMathLibrary.Conv_IntToBool` (`KismetArrayLibrary.Array_Length` (`self.GetOverlappingActors` (`ChildActorComponent.ChildActor` (`self.BP_RoomCollider`)) "/Game/DungeonGenerator/SubLevels/Blueprint/BP_RoomCollider.BP_RoomCollider_C")))))

(fn `GetConnectionPointWithState`
  (params (State :type "/Game/DungeonGenerator/SubLevels/Blueprint/ConnectionPointState Enum" :default "NewEnumerator0"))
  (returns (ConnectionPoints :type "Array of /Game/DungeonGenerator/SubLevels/Blueprint/BP_ConnectionPoint Object Reference"))
  (`KismetArrayLibrary.Array_Clear` (`self.AllConnectionPointsWithState`))
  (for _array_element (`self.AllConnectionPoints`)
    (if (`|EnumEquality` (`/Game/DungeonGenerator/SubLevels/Blueprint/BP_ConnectionPoint.State` _array_element) State)
      (`KismetArrayLibrary.Array_Add` (`self.AllConnectionPointsWithState`) _array_element)))
  (return (`self.AllConnectionPointsWithState`)))

(fn `UserConstructionScript`
  (locals (SizeX :type "Float (double-precision)") (SizeY :type "Float (double-precision)"))
  (bind _returnvalue (`self.GetTransform` self))
  (set `self.SizeX` (* (.x (.location (`SceneComponent.GetRelativeTransform` (`self.BP_ConnectionPointNorth00`)))) (.x (.scale _returnvalue))))
  (set `self.SizeY` (* (.y (.location (`SceneComponent.GetRelativeTransform` (`self.BP_ConnectionPointEst00`)))) (.y (.scale _returnvalue))))
  (`|ExecutionSequence`
    (:`then_0`
      (`/Game/DungeonGenerator/SubLevels/Blueprint/BP_ConnectionPoint.ChangeState` (cast `/Game/DungeonGenerator/SubLevels/Blueprint/BP_ConnectionPoint` (`ChildActorComponent.ChildActor` (`self.BP_ConnectionPointNorth00`)) :!pure true) (`self.CP_N_00`))
      (`/Game/DungeonGenerator/SubLevels/Blueprint/BP_ConnectionPoint.ChangeState` (cast `/Game/DungeonGenerator/SubLevels/Blueprint/BP_ConnectionPoint` (`ChildActorComponent.ChildActor` (`self.BP_ConnectionPointSouth00`)) :!pure true) (`self.CP_S_00`))
      (`/Game/DungeonGenerator/SubLevels/Blueprint/BP_ConnectionPoint.ChangeState` (cast `/Game/DungeonGenerator/SubLevels/Blueprint/BP_ConnectionPoint` (`ChildActorComponent.ChildActor` (`self.BP_ConnectionPointEst00`)) :!pure true) (`self.CP_E_00`))
      (`/Game/DungeonGenerator/SubLevels/Blueprint/BP_ConnectionPoint.ChangeState` (cast `/Game/DungeonGenerator/SubLevels/Blueprint/BP_ConnectionPoint` (`ChildActorComponent.ChildActor` (`self.BP_ConnectionPointWest00`)) :!pure true) (`self.CP_W_00`)))
    (:`then_1`
      (`/Game/DungeonGenerator/SubLevels/Blueprint/BP_ConnectionPoint.ChangeState` (cast `/Game/DungeonGenerator/SubLevels/Blueprint/BP_ConnectionPoint` (`ChildActorComponent.ChildActor` (`self.BP_ConnectionPointNorth01`)) :!pure true) (`self.CP_N_01`))
      (`/Game/DungeonGenerator/SubLevels/Blueprint/BP_ConnectionPoint.ChangeState` (cast `/Game/DungeonGenerator/SubLevels/Blueprint/BP_ConnectionPoint` (`ChildActorComponent.ChildActor` (`self.BP_ConnectionPointSouth01`)) :!pure true) (`self.CP_S_01`))
      (`/Game/DungeonGenerator/SubLevels/Blueprint/BP_ConnectionPoint.ChangeState` (cast `/Game/DungeonGenerator/SubLevels/Blueprint/BP_ConnectionPoint` (`ChildActorComponent.ChildActor` (`self.BP_ConnectionPointEst01`)) :!pure true) (`self.CP_E_01`))
      (`/Game/DungeonGenerator/SubLevels/Blueprint/BP_ConnectionPoint.ChangeState` (cast `/Game/DungeonGenerator/SubLevels/Blueprint/BP_ConnectionPoint` (`ChildActorComponent.ChildActor` (`self.BP_ConnectionPointWest01`)) :!pure true) (`self.CP_W_01`)))
    (:`then_2`
      (`/Game/DungeonGenerator/SubLevels/Blueprint/BP_ConnectionPoint.ChangeState` (cast `/Game/DungeonGenerator/SubLevels/Blueprint/BP_ConnectionPoint` (`ChildActorComponent.ChildActor` (`self.BP_ConnectionPointNorth02`)) :!pure true) (`self.CP_N_02`))
      (`/Game/DungeonGenerator/SubLevels/Blueprint/BP_ConnectionPoint.ChangeState` (cast `/Game/DungeonGenerator/SubLevels/Blueprint/BP_ConnectionPoint` (`ChildActorComponent.ChildActor` (`self.BP_ConnectionPointSouth02`)) :!pure true) (`self.CP_S_02`))
      (`/Game/DungeonGenerator/SubLevels/Blueprint/BP_ConnectionPoint.ChangeState` (cast `/Game/DungeonGenerator/SubLevels/Blueprint/BP_ConnectionPoint` (`ChildActorComponent.ChildActor` (`self.BP_ConnectionPointEst02`)) :!pure true) (`self.CP_E_02`))
      (`/Game/DungeonGenerator/SubLevels/Blueprint/BP_ConnectionPoint.ChangeState` (cast `/Game/DungeonGenerator/SubLevels/Blueprint/BP_ConnectionPoint` (`ChildActorComponent.ChildActor` (`self.BP_ConnectionPointWest02`)) :!pure true) (`self.CP_W_02`)))
    (:`then_3`
      (bind _output_get (set `self.AllConnectionPoints` (`|MakeArray` (cast `/Game/DungeonGenerator/SubLevels/Blueprint/BP_ConnectionPoint` (`ChildActorComponent.ChildActor` (`self.BP_ConnectionPointNorth00`)) :!pure true) (cast `/Game/DungeonGenerator/SubLevels/Blueprint/BP_ConnectionPoint` (`ChildActorComponent.ChildActor` (`self.BP_ConnectionPointSouth00`)) :!pure true) (cast `/Game/DungeonGenerator/SubLevels/Blueprint/BP_ConnectionPoint` (`ChildActorComponent.ChildActor` (`self.BP_ConnectionPointEst00`)) :!pure true) (cast `/Game/DungeonGenerator/SubLevels/Blueprint/BP_ConnectionPoint` (`ChildActorComponent.ChildActor` (`self.BP_ConnectionPointWest00`)) :!pure true) (cast `/Game/DungeonGenerator/SubLevels/Blueprint/BP_ConnectionPoint` (`ChildActorComponent.ChildActor` (`self.BP_ConnectionPointNorth01`)) :!pure true) (cast `/Game/DungeonGenerator/SubLevels/Blueprint/BP_ConnectionPoint` (`ChildActorComponent.ChildActor` (`self.BP_ConnectionPointSouth01`)) :!pure true) (cast `/Game/DungeonGenerator/SubLevels/Blueprint/BP_ConnectionPoint` (`ChildActorComponent.ChildActor` (`self.BP_ConnectionPointEst01`)) :!pure true) (cast `/Game/DungeonGenerator/SubLevels/Blueprint/BP_ConnectionPoint` (`ChildActorComponent.ChildActor` (`self.BP_ConnectionPointWest01`)) :!pure true) (cast `/Game/DungeonGenerator/SubLevels/Blueprint/BP_ConnectionPoint` (`ChildActorComponent.ChildActor` (`self.BP_ConnectionPointNorth02`)) :!pure true) (cast `/Game/DungeonGenerator/SubLevels/Blueprint/BP_ConnectionPoint` (`ChildActorComponent.ChildActor` (`self.BP_ConnectionPointSouth02`)) :!pure true) (cast `/Game/DungeonGenerator/SubLevels/Blueprint/BP_ConnectionPoint` (`ChildActorComponent.ChildActor` (`self.BP_ConnectionPointEst02`)) :!pure true) (cast `/Game/DungeonGenerator/SubLevels/Blueprint/BP_ConnectionPoint` (`ChildActorComponent.ChildActor` (`self.BP_ConnectionPointWest02`)) :!pure true))))
      (for _array_element _output_get
        (set `/Game/DungeonGenerator/SubLevels/Blueprint/BP_ConnectionPoint.SizeX` (`local.SizeX`) _array_element)
        (set `/Game/DungeonGenerator/SubLevels/Blueprint/BP_ConnectionPoint.SizeY` (`local.SizeY`) _array_element)))))