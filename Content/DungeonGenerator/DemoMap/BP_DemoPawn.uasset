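; Demo pawn that drives the DungeonBuilder plugin through number-key shortcuts in the dungeon generator demo map.
; On BeginPlay it caches the first DungeonBuilder actor in the level.
; Keys trigger clearing sublevels, building with a random or fixed seed, and saving or loading the dungeon in a disk slot.
; Clear, random build, save and load bind completion events that print status messages; the fixed-seed build binds none.
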(event `self.ReceiveBeginPlay`
  ;[1 1 1] We Get the DungeonBuilder Blueprint
  (bind _outactors (`GameplayStatics.GetAllActorsOfClass` "/Game/DungeonGenerator/Generator/DungeonBuilder.DungeonBuilder_C"))
  (set `self.DungeonBuilder` (`|GetArrayItem` _outactors)))

(event `Key|One`
  (params (Key :type "Key Structure"))
  (:`Pressed`
    ;[1 1 1] We Bind on Clear Done Event
    (add `/Game/DungeonGenerator/Generator/DungeonBuilder.OnClearDone` (`self.DungeonBuilder`) (delegate `ClearDone`))
    ;[1 1 1] We Clear the SubLevels
    (`/Game/DungeonGenerator/Generator/DungeonBuilder.CleanSubLevels` (`self.DungeonBuilder`))))

(event `ClearDone`
  ;[1 1 1] We Bind on Clear Done Event
  (`KismetSystemLibrary.PrintString` "Dungeon is Cleared."))

(event `Key|Two`
  (params (Key :type "Key Structure"))
  (:`Pressed`
    ;[1 1 1] We bind to ConstructionDone Event
    (add `/Game/DungeonGenerator/Generator/DungeonBuilder.OnConstructionDone` (`self.DungeonBuilder`) (delegate `StartGame`))
    ;[1 1 1] We Build The Dungeon
    (set `/Game/DungeonGenerator/Generator/DungeonBuilder.UseRandomSeed` true (`self.DungeonBuilder`))
    (`/Game/DungeonGenerator/Generator/DungeonBuilder.BuildDungeon` (`self.DungeonBuilder`))))

(event `StartGame`
  ;[1 1 1] Dungeon Is built we can proceed with the rest of the game logic
  (`KismetSystemLibrary.PrintString` "Dungeon is Ready."))

(event `Key|Three`
  (params (Key :type "Key Structure"))
  (:`Pressed`
    ;[1 1 1] We Bind on Dungeon Saved Event
    (add `/Game/DungeonGenerator/Generator/DungeonBuilder.OnDungeonSaved` (`self.DungeonBuilder`) (delegate `DungeonSaved`))
    ;[1 1 1] We Save to Level
    (`/Game/DungeonGenerator/Generator/DungeonBuilder.SaveLevelToDisk` (`self.DungeonBuilder`) "Slot1")))

(event `DungeonSaved`
  ;[1 1 1] We Bind on Dungeon Saved Event
  (`KismetSystemLibrary.PrintString` "Dungeon Saved in Slot1"))

(event `Key|Four`
  (params (Key :type "Key Structure"))
  (:`Pressed`
    ;[1 1 1] We Bind on Load Done Event
    (add `/Game/DungeonGenerator/Generator/DungeonBuilder.OnLoadDone` (`self.DungeonBuilder`) (delegate `LoadingDone`))
    ;[1 1 1] We Load the level
    (`/Game/DungeonGenerator/Generator/DungeonBuilder.LoadLevelFromDisk` (`self.DungeonBuilder`) "Slot1")))

(event `LoadingDone`
  ;[1 1 1] We Bind on Load Done Event
  (`KismetSystemLibrary.PrintString` "Dungeon Loaded from Slot1"))

(event `Key|Five`
  (params (Key :type "Key Structure"))
  (:`Pressed`
    ;[1 1 1] We Build The Dungeon
    (set `/Game/DungeonGenerator/Generator/DungeonBuilder.UseRandomSeed` false (`self.DungeonBuilder`))
    (`/Game/DungeonGenerator/Generator/DungeonBuilder.BuildDungeon` (`self.DungeonBuilder`))))

(fn `UserConstructionScript`)